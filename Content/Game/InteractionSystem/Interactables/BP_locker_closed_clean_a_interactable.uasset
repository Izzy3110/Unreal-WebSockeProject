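; Interactable locker Blueprint whose door opens and closes when an actor interacts with it.
; The Interact event toggles on the IsOpen flag, calling OpenDoor or CloseDoor.
; Each plays its own timeline from the start to drive the door mesh's yaw rotation.
; An optional DebugInteraction flag prints the interactable and interactor names.
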(event `Open Door`
  (set `self.IsOpen?` true)
  (bind (_direction _zrotation) (`Timeline|TL_OpenDoor` :!via `PlayFromStart`)
    (:`Update`
      (`SceneComponent.K2_SetRelativeRotation` (`self.SM_locker_0001_door`) (`KismetMathLibrary.MakeRotator` 0.0 0.0 _zrotation) false false))))

(event `Close Door`
  (set `self.IsOpen?` false)
  (bind (_direction _zrotation) (`Timeline|TL_CloseDoor` :!via `PlayFromStart`)
    (:`Update`
      (`SceneComponent.K2_SetRelativeRotation` (`self.SM_locker_0001_door`) (`KismetMathLibrary.MakeRotator` 0.0 0.0 _zrotation) false false))))

(event `/Game/Game/InteractionSystem/BPI_Interaction.Interact`
  (params (Interactor :type "Actor Object Reference"))
  (if (`self.DebugInteraction`)
    (`KismetSystemLibrary.PrintString` (`KismetTextLibrary.Conv_TextToString` (`|FormatText` "Interactable: {Interactable}" (`KismetSystemLibrary.GetDisplayName` self))))
    (`KismetSystemLibrary.PrintString` "Interacting...")
    (`KismetSystemLibrary.PrintString` (`KismetTextLibrary.Conv_TextToString` (`|FormatText` "Interactor: {Interactor}" (`KismetSystemLibrary.GetDisplayName` Interactor)))))
  (if (not (`self.IsOpen?`))
    (`self.Open Door`)
    (else
      (`self.Close Door`))))

(fn `UserConstructionScript`)