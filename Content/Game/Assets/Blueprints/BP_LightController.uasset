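; Light controller actor that recolors its directional lights from a list of colors.
; On BeginPlay, GetLights gathers every DirectionalLight component under the root, printing "Failed" for other child types.
; SetRandomColor, not called within this Blueprint, colors the lights passed in, or DirectionalLightMM if none.
; Despite its name, it cycles colors in order, advancing a shared wrapping index after each light.
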(event `self.ReceiveBeginPlay`
  (bind _result_components (`self.GetLights`))
  (set `self.LightComponents` _result_components))

(event `self.ReceiveTick`
  (params (DeltaSeconds :type "Float (single-precision)")))

(fn `GetLights`
  (returns (`Result Components` :type "Array of LightComponent Object Reference"))
  (locals (`Current LightComponents` :type "Array of LightComponent Object Reference"))
  (for _array_element (`SceneComponent.GetChildrenComponents` (`self.DefaultSceneRoot`) true)
    (bind _asdirectional_light_component (cast `DirectionalLightComponent` _array_element)
      (:`then`
        (`KismetArrayLibrary.Array_AddUnique` (`self.LightComponents`) _asdirectional_light_component))
      (:`CastFailed`
        (`KismetSystemLibrary.PrintString` "Failed"))))
  (return (`self.LightComponents`)))

(fn `SetRandomColor`
  (params (TargetLights :type "Array of LightComponent Object Reference"))
  (locals (Target :type "LightComponent Object Reference"))
  ;[0 1 0.03912 0.5] Default to Single Light if no Light Component in Array
  (if (== (`KismetArrayLibrary.Array_Length` TargetLights) 0)
    (set `local.Target` (`self.DirectionalLight_MM`))
    ;[0 1 0.03912 0.5] Set Next Color of Target Light
    (`LightComponent.SetLightColor` (`local.Target`) (`KismetMathLibrary.Conv_ColorToLinearColor` (`|GetArrayItem` (`self.Colors`) (`self.Current Color I`))) true :!label _label)
    ;[0 1 0.03912 0.5] If Less than (Colors.len -1)
    (if (< (`self.Current Color I`) (- (`KismetArrayLibrary.Array_Length` (`self.Colors`)) 1))
      ;[0 1 0.03912 0.5] Increment | else | Rewind Index to Start
      (bind _result (`/Engine/EditorBlueprintResources/StandardMacros.IncrementInt` (`self.Current Color I`))
        (:`  `
          (set `self.Current Color I` _result)))
      (else
        (set `self.Current Color I` 0)))
    (else
      (for _array_element TargetLights
        (set `local.Target` _array_element)
        (goto _label)))))

(fn `UserConstructionScript`)