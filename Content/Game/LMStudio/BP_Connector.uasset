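; Connector actor that links an in-game AI chat UI to an LM Studio server.
; On BeginPlay it creates the chat and input widgets, initializes and tests the connector, and runs debug YAML tests on hardcoded local files.
; ExecuteRequest posts JSON to the server's /responses endpoint through an async request node.
; AddMessage shows requests, results and connection status as colored message widgets in the chat.
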(event `self.ReceiveBeginPlay`
  (bind _lmstudioconnector (`self.LMStudioConnector`))
  (`|ExecutionSequence`
    (:`then_0`
      (bind _returnvalue (`|CreateWidget` "/Game/Game/LMStudio/WBP_AIChat.WBP_AIChat_C"))
      (bind _output_get (set `self.WBP_AIChat` _returnvalue))
      (`UserWidget.AddToViewport` _output_get 0))
    (:`then_1`
      (bind _returnvalue_2 (`|GenericCreateObject` "/Game/Game/LMStudio/MyLMStudioConnector.MyLMStudioConnector_C"))
      (bind _output_get_2 (set `self.LMStudioConnector` _returnvalue_2))
      (`LMStudioConnector.InitializeFromSettings` _output_get_2)
      (`LMStudioConnector.PrintSettings` _lmstudioconnector)
      (`LMStudioConnector.TestServerConnection` _lmstudioconnector (delegate `OnTestServerCompleted`)))
    (:`then_2`
      (bind _returnvalue_3 (`|CreateWidget` "/Game/Game/LMStudio/WBP_AIChat_Input.WBP_AIChat_Input_C"))
      (bind _output_get_3 (set `self.WBP_AIChat_Input` _returnvalue_3))
      (set `/Game/Game/LMStudio/WBP_AIChat_Input.BP_Connector` self _output_get_3)
      (`UserWidget.AddToViewport` (`self.WBP_AIChat_Input`) 0))
    (:`then_3`
      (bind (_bsuccess _log) (`YamlTestLibrary.TestPromptsYaml` "C:\\Users\\sasch\\AppData\\Roaming\\WebSockeProject\\Tests\\LMStudio\\Tests.Prompts.yaml"))
      (if _bsuccess
        (`KismetSystemLibrary.PrintString` "SUCCESS")
        (else
          (`KismetSystemLibrary.PrintString` "FAILED")))
      (`KismetSystemLibrary.PrintString` _log))
    (:`then_4`
      (bind (_bsuccess_2 _log_2) (`YamlTestLibrary.TestResponsesYaml` "C:\\Users\\sasch\\AppData\\Roaming\\WebSockeProject\\Tests\\LMStudio\\Tests.Responses.yaml"))
      (if _bsuccess_2
        (`KismetSystemLibrary.PrintString` "SUCCESS")
        (else
          (`KismetSystemLibrary.PrintString` "FAILED")))
      (`KismetSystemLibrary.PrintString` _log_2))
    (:`then_5`
      (bind (_jsonoutput _bsuccess_3 _errormessage) (`YamlBlueprintLibrary.LoadYamlFromFile` "C:\\Users\\sasch\\AppData\\Roaming\\WebSockeProject\\Tests\\LMStudio\\Tests.Responses.yaml"))
      (if _bsuccess_3
        (`KismetSystemLibrary.PrintString` "SUCCESS")
        (else
          (`KismetSystemLibrary.PrintString` "FAILED")
          (`KismetSystemLibrary.PrintString` _errormessage)))
      (`KismetSystemLibrary.PrintString` (`KismetTextLibrary.Conv_TextToString` (`|FormatText` "JSON: {Json Output}" _jsonoutput)))
      (bind (_values _bsuccess_4) (`YamlBlueprintLibrary.GetValuesFromYamlPathWithFilters` _jsonoutput "output.content.text" (`|MakeMap` "output.content.type" "output_text")))
      (if _bsuccess_4
        (`KismetSystemLibrary.PrintString` (`KismetTextLibrary.Conv_TextToString` (`|FormatText` "SUCCESS: GetValuesFromYamlPath")) true true (struct :`R` 1.0 :`G` 0.574419 :`A` 1.0) 30.0)
        (`KismetSystemLibrary.PrintString` (`KismetTextLibrary.Conv_TextToString` (`|FormatText` "LEN: {Length}" (`KismetArrayLibrary.Array_Length` _values))) true true (struct :`R` 0.905411 :`G` 1.0 :`B` 0.045618 :`A` 1.0) 30.0)
        (for _array_element _values
          (`KismetSystemLibrary.PrintText` (`|FormatText` "OUTPUT: {OUTPUT TEXT}" _array_element) true true (struct :`G` 0.423131 :`B` 1.0 :`A` 1.0) 30.0))
        (else
          (`KismetSystemLibrary.PrintString` (`KismetTextLibrary.Conv_TextToString` (`|FormatText` "FAILED: GetValuesFromYamlPath")) true true (struct :`R` 1.0 :`B` 0.76972 :`A` 1.0) 30.0))))))

(event `OnTestServerCompleted`
  (params (bSuccess :type Boolean))
  (if bSuccess
    (`KismetSystemLibrary.PrintString` "LMStudio: Server-Connection-Test: Success" true true (struct :`R` 0.551033 :`G` 1.0 :`B` 0.274397 :`A` 1.0) 5.0)
    (`self.AddMessage` "LMStudio: Server-Connection-Test: Success" (struct :`R` 0.352082 :`G` 1.0 :`B` 0.397225 :`A` 1.0))
    (set `self.bLMStudio_Ready` true)
    (else
      (`KismetSystemLibrary.PrintString` "LMStudio: Server-Connection-Test: Failed" true true (struct :`R` 1.0 :`G` 0.048685 :`B` 0.096454 :`A` 1.0) 10.0)
      (`self.AddMessage` "LMStudio: Server-Connection-Test: Failed")
      (set `self.bLMStudio_Ready` false))))

(event `Execute Request`
  (params (InputJSON :type String))
  (bind _returnvalue (`KismetStringLibrary.Concat_StrStr` (`LMStudioConnector.ServerBaseURL` (`self.LMStudioConnector`)) "/responses"))
  (`self.AddMessage` InputJSON (struct :`R` 0.383021 :`G` 1.0 :`B` 0.101042 :`A` 1.0))
  (`self.AddMessage` _returnvalue)
  (bind (_responsecontent _errormessage) (`LMStudioRequest.SendLMStudioRequest` _returnvalue "lm-studio" InputJSON)
    (:`OnSuccess`
      (`self.AddMessage` "success" (struct :`R` 0.166008 :`G` 1.0 :`B` 0.396116 :`A` 1.0))
      (`self.AddMessage` _responsecontent (struct :`R` 0.383151 :`G` 1.0 :`B` 0.202937 :`A` 1.0))
      (`KismetSystemLibrary.PrintString` _responsecontent)
      (`KismetSystemLibrary.PrintString` InputJSON))
    (:`OnFailure`
      (`self.AddMessage` "fail" (struct :`R` 1.0 :`G` 0.23524 :`B` 0.378928 :`A` 1.0))
      (`self.AddMessage` _errormessage (struct :`R` 1.0 :`G` 0.09255 :`B` 0.083956 :`A` 1.0)))))

(fn `AddMessage`
  (params (Text :type String) (Color :type "LinearColor Structure" :default (struct :`R` 1.0 :`G` 1.0 :`B` 1.0 :`A` 1.0)))
  (locals (NewMessage :type "/Game/Game/LMStudio/WBP_AIChat_Message Object Reference") (DefaultColor :type "LinearColor Structure" :default (struct :`R` 1.0 :`G` 1.0 :`B` 1.0 :`A` 1.0)))
  (bind _wbp_aichat (`self.WBP_AIChat`)
    (:`then`
      (bind _returnvalue (`|CreateWidget` "/Game/Game/LMStudio/WBP_AIChat_Message.WBP_AIChat_Message_C"))
      (bind _output_get (set `local.NewMessage` _returnvalue))
      (set `/Game/Game/LMStudio/WBP_AIChat_Message.ChatMessage_TextValue` Text _output_get)
      (if (!= Color (`local.DefaultColor`))
        (`TextBlock.SetColorAndOpacity` (`/Game/Game/LMStudio/WBP_AIChat_Message.ChatMessage_Text` (`local.NewMessage`)) (make `SlateColor` (`local.Color`)))
        (else
          (`TextBlock.SetColorAndOpacity` (`/Game/Game/LMStudio/WBP_AIChat_Message.ChatMessage_Text` (`local.NewMessage`)) (make `SlateColor` (`local.DefaultColor`)))))
      (`VerticalBox.AddChildToVerticalBox` (`/Game/Game/LMStudio/WBP_AIChat.MessageBox_VerticalBox` _wbp_aichat) (`local.NewMessage`)))
    (:`else`)))

(fn `UserConstructionScript`)