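; Observer actor that reports the yaw of a tagged BP_Rotator over a WebSocket as JSON event/payload messages.
; BeginPlay caches the game instance's WebSocket client and sends one message after a short delay.
; Tick reads the rotator's root rotation and sends yaw every frame via ConstructJSON while connected.
; A time-throttled send using LastReport and DiffMax exists but is unwired, so sending is unthrottled.
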(event `self.ReceiveBeginPlay`
  (bind _currentjson (`self.CurrentJSON`))
  (bind (_rotation_roll _rotation_pitch _rotation_yaw) (`KismetMathLibrary.BreakRotator` (`self.Rotation`)))
  (bind _asmain_game_instance (cast `/Game/MainGameInstance` (`GameplayStatics.GetGameInstance`)))
  (set `self.As My Blueprint Web Socket Client` (`/Game/MainGameInstance.MyWsBP` _asmain_game_instance))
  (`KismetSystemLibrary.Delay` 2.0)
  (`/Engine/EditorBlueprintResources/StandardMacros.IsValid` (`self.As My Blueprint Web Socket Client`)
    (:`Is Valid`
      (`KismetSystemLibrary.PrintString` "valid!")
      (if (`BlueprintWebSocketClient.IsConnected` (`self.As My Blueprint Web Socket Client`))
        (`KismetSystemLibrary.PrintString` "Connected")
        (set `self.CurrentJSON` (make `JsonObjectWrapper`))
        (`|SetJsonField` _currentjson "event" "message")
        (`|SetJsonField` _currentjson "payload" (`KismetStringLibrary.Conv_DoubleToString` _rotation_yaw))
        (bind _outjsonstring (`JsonBlueprintFunctionLibrary.ToString` (`self.CurrentJSON`)))
        (`KismetSystemLibrary.PrintString` _outjsonstring)
        (`BlueprintWebSocketClient.SendMessage` (`self.As My Blueprint Web Socket Client`) _outjsonstring)
        (else
          (`KismetSystemLibrary.PrintString` "Not Connected"))))
    (:`Is Not Valid`
      (`KismetSystemLibrary.PrintString` "not valid"))))

(event `self.ReceiveTick`
  (params (DeltaSeconds :type "Float (single-precision)"))
  (bind (_rotation_roll _rotation_pitch _rotation_yaw) (`KismetMathLibrary.BreakRotator` (`self.Rotation`)))
  (bind _returnvalue (`GameplayStatics.GetActorOfClass` "/Game/BP_Rotator.BP_Rotator_C"))
  (if (`self.ActorHasTag` _returnvalue "Rotator")
    (`KismetSystemLibrary.PrintString` "found")
    (bind _output_get (set `self.BP Rotator` _returnvalue))
    (set `self.Rotation` (`SceneComponent.K2_GetComponentRotation` (`/Game/BP_Rotator.DefaultSceneRoot` _output_get)))
    (`/Engine/EditorBlueprintResources/StandardMacros.IsValid` (`self.As My Blueprint Web Socket Client`)
      (:`Is Valid`
        (`KismetSystemLibrary.PrintString` "valid!")
        (if (`BlueprintWebSocketClient.IsConnected` (`self.As My Blueprint Web Socket Client`))
          (`KismetSystemLibrary.PrintString` "Connected")
          (bind _jsonstr (`self.ConstructJSON` "message" (`KismetStringLibrary.Conv_DoubleToString` _rotation_yaw)))
          (`BlueprintWebSocketClient.SendMessage` (`self.As My Blueprint Web Socket Client`) _jsonstr)
          (else
            (`KismetSystemLibrary.PrintString` "Not Connected"))))
      (:`Is Not Valid`
        (`KismetSystemLibrary.PrintString` "not valid")))))

(fn `ConstructJSON`
  (params (EventValue :type String :default "message") (Payload :type String))
  (returns (JsonStr :type String) (Success :type Boolean))
  (locals (LocalJSON :type "JsonObjectWrapper Structure"))
  (bind _localjson (`local.LocalJSON`))
  (set `local.LocalJSON` (make `JsonObjectWrapper`))
  (`|SetJsonField` _localjson "event" (`KismetSystemLibrary.MakeLiteralString` EventValue))
  (`|SetJsonField` _localjson "payload" Payload)
  (bind (_outjsonstring _returnvalue) (`JsonBlueprintFunctionLibrary.ToString` (`local.LocalJSON`)))
  (return _outjsonstring _returnvalue))

(fn `UpdateLastReport`
  (set `self.last_report` (`KismetMathLibrary.ToUnixTimestamp` (`KismetMathLibrary.Now`))))

(fn `UserConstructionScript`)